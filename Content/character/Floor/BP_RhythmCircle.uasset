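; BP_RhythmCircle is a floor circle actor that lights up with a colored glow, likely as a rhythm indicator.
; On BeginPlay it creates a dynamic material instance on its Plane, turns the glow off, then after a one-second delay fires a purple test pulse.
; PlayPulse takes a color and sets the material's CircleColor and raises GlowPower, with no fade back down.
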(event EventBeginPlay
  (bind _returnvalue (Rendering|Material|CreateDynamicMaterialInstance (Variables|Default|GetPlane) 0 0 "None" :!class /Script/Engine.PrimitiveComponent))
  (bind _output_get (Variables|Default|SetCircleMat _returnvalue))
  (Rendering|Material|SetScalarParameterValue _output_get "GlowPower" 0.0 :!class /Script/Engine.MaterialInstanceDynamic)
  (Utilities|FlowControl|Delay 1.0)
  (CallFunction|PlayPulse (Utilities|Struct|MakeLinearColor 0.8 0.2 1.0 1.0)))

(event Collision|EventActorBeginOverlap
  (params (OtherActor :type Actor%20Object%20Reference)))

(event EventTick
  (params (DeltaSeconds :type Float%20%28single-precision%29)))

(fn ConstructionScript)

(fn PlayPulse
  (params (NewColor :type Linear%20Color%20Structure))
  (bind _circlemat (Variables|Default|GetCircleMat))
  (Rendering|Material|SetVectorParameterValue _circlemat "CircleColor" NewColor :!class /Script/Engine.MaterialInstanceDynamic)
  (Rendering|Material|SetScalarParameterValue _circlemat "GlowPower" 1e+01 :!class /Script/Engine.MaterialInstanceDynamic))